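; Base enemy Blueprint that tracks health and death.
; Health starts at DefaultHealth in the construction script; AnyDamage lowers it with clamping and, at zero, sets BIsDead and calls EnemyDied once.
; EnemyDied is an empty function in this class.
; Separately, a capsule overlap with a BP_Projectile destroys the enemy immediately, bypassing both health and EnemyDied.
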(event `self.ReceiveAnyDamage`
  (params (Damage :type "Float (single-precision)") (DamageType :type "DamageType Object Reference") (InstigatedBy :type "Controller Object Reference") (DamageCauser :type "Actor Object Reference"))
  (set `self.Health` (`KismetMathLibrary.FClamp` (- (`self.Health`) Damage) 0.0 (`self.DefaultHealth`)))
  (if (and (<= (`self.Health`) 0.0) (not (`self.BIsDead`)))
    (set `self.BIsDead` true)
    (`self.EnemyDied`)))

(event `self.CapsuleComponent.OnComponentBeginOverlap`
  (params (OverlappedComponent :type "PrimitiveComponent Object Reference") (OtherActor :type "Actor Object Reference") (OtherComp :type "PrimitiveComponent Object Reference") (OtherBodyIndex :type Integer) (bFromSweep :type Boolean) (SweepResult :type "HitResult Structure (by ref)"))
  ;[1 1 1] Enemy Destruction from Projectile
  (cast `/Game/Content/Blueprint/Interactives/BP_Projectile` OtherActor)
  (`self.K2_DestroyActor`))

(fn `EnemyDied`)

(fn `UserConstructionScript`
  (set `self.Health` (`self.DefaultHealth`)))